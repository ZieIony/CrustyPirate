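; Platform Blueprint that is solid and visible only while the player's feet are above it, acting as a one-way platform.
; Every tick, UpdateCollision compares the bottom of player 0's capsule with the platform's actor Z plus a fixed offset.
; The result switches RenderComponent between Block and Ignore on a custom trace channel, and also shows or hides that component.
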(event EventTick
  (params (DeltaSeconds :type Float%20%28single-precision%29))
  (CallFunction|UpdateCollision))

(fn ConstructionScript)

(fn UpdateCollision
  (bind _returnvalue (Game|GetPlayerCharacter 0))
  (bind _returnvalue_2 (Transformation|GetActorLocation))
  (bind _returnvalue_3 (Transformation|GetActorLocation _returnvalue))
  (bind _returnvalue_4 (+ (.z _returnvalue_2) 32.0))
  (bind _capsulecomponent (Variables|/Script/Engine.Character|GetCapsuleComponent _returnvalue))
  (bind _returnvalue_5 (Components|Capsule|GetScaledCapsuleHalfHeight _capsulecomponent))
  (bind _returnvalue_6 (- (.z _returnvalue_3) _returnvalue_5))
  (bind _returnvalue_7 (> _returnvalue_6 _returnvalue_4))
  (Collision|SetCollisionResponsetoChannel (Variables|Default|GetRenderComponent) "ECC_GameTraceChannel1" (select _returnvalue_7 "ECR_Block" "ECR_Ignore"))
  (Rendering|SetVisibility (Variables|Default|GetRenderComponent) _returnvalue_7 false))