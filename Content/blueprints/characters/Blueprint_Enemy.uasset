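; Enemy character Blueprint that keeps its on-screen health bar in sync with its health.
; On BeginPlay it binds to its health-changed event.
; Each change casts the HealthBar component's widget to EnemyHealthBar and passes it the new health and max hit points.
; The bar is hidden when health reaches exactly zero and shown otherwise.
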(event Custom|OnHealthChanged
  (params (NewHealth :type Float%20%28single-precision%29))
  (bind _asenemy_health_bar (Utilities|Casting|CastToEnemyHealthBar (UserInterface|GetUserWidgetObject (Variables|Default|GetHealthBar))))
  (Class|EnemyHealthBar|SetHealth _asenemy_health_bar NewHealth (Math|Conversions|ToFloat(Integer) (Variables|Default|GetMaxHitPoints)))
  (Development|SetHiddeninGame (Variables|Default|GetHealthBar) (== NewHealth 0.0) false))

(event EventBeginPlay
  (EventDispatchers|BindEventtoOnHealthChangedEvent (delegate Custom|OnHealthChanged)))

(fn ConstructionScript)